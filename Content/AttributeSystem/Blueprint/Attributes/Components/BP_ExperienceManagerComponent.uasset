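; Actor component that manages named experience types, each with an amount, level, optional max level and LevelModifier curve for required experience.
; Loaded experiences are kept in a backup map, from which the live map is built or individually reset, with Server_ events wrapping the edit functions.
; Amount changes loop overflow across levels.
; Direct level edits fire increased, decreased, min and max dispatchers, which amount-driven level changes skip.
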(event Custom|Server_BuildExperiences
  ;[0.9734 0.1356 0.1356] Server: Base Experience List
  ;;[1 1 1 0.498] Server: Experience Base Events
  (Interface|Experience|BuildExperiences))

(event Custom|Server_SetExperienceLevelModifier
  (params (Experience :type String) (LevelModifier :type Curve%20Float%20Object%20Reference))
  ;[0.9734 0.1356 0.1356] Server: Experience Events
  ;;[1 1 1 0.498] Level Modifier
  (Interface|Experience|SetExperienceLevelModifier Experience LevelModifier))

(event Custom|Event_InitializeExperienceManager
  (params (Experiences :type Map%20of%20Strings%20to%20Structs))
  ;[0.3916 1 0.3372] Event: Initialize Experience Bars
  (Manager|Public|InitializeExperienceManager Experiences))

(event Custom|Server_ModifyExperienceLevel
  (params (Experience :type String) (Calculation :type CalculationType%20Enum :default "NewEnumerator0") (Amount :type Integer))
  ;[0.9734 0.1356 0.1356] Server: Experience Events
  ;;[1 1 1 0.498] Experience Level
  (Interface|Experience|ModifyExperienceLevel Experience Calculation Amount))

(event Custom|Server_ModifyExperienceAmount
  (params (Experience :type String) (Calculation :type CalculationType%20Enum :default "NewEnumerator0") (Amount :type Integer))
  ;[0.9734 0.1356 0.1356] Server: Experience Events
  ;;[1 1 1 0.498] Experience Amount
  (Interface|Experience|ModifyExperienceAmount Experience Calculation Amount))

(event Custom|Server_SetExperienceLevel
  (params (Experience :type String) (Amount :type Integer))
  ;[0.9734 0.1356 0.1356] Server: Experience Events
  ;;[1 1 1 0.498] Experience Level
  (Interface|Experience|SetExperienceLevel Experience Amount))

(event Custom|Event_LoadExperiences
  (params (Experiences :type Map%20of%20Strings%20to%20Structs))
  ;[0.9734 0.1356 0.1356] Event: Load Experiences
  (Manager|Public|LoadExperiences Experiences))

(event Custom|Server_SetExperienceAmount
  (params (Experience :type String) (Amount :type Integer))
  ;[0.9734 0.1356 0.1356] Server: Experience Events
  ;;[1 1 1 0.498] Experience Amount
  (Interface|Experience|SetExperienceAmount Experience Amount))

(event Custom|Server_BuildSpecificExperience
  (params (ExperienceType :type String))
  ;[0.9734 0.1356 0.1356] Server: Base Experience List
  ;;[1 1 1 0.498] Server: Experience Base Events
  (Interface|Experience|BuildSpecificExperience ExperienceType))

(event Custom|Server_AddExperience
  (params (ExperienceType :type String) (Values :type Experience%20List%20Structure%20%28by%20ref%29))
  ;[0.9734 0.1356 0.1356] Server: Base Experience List
  ;;[1 1 1 0.498] Server: Experience Base Events
  (Manager|Private|Maps|Add|AddExperience ExperienceType Values))

(event Custom|Server_RemoveExperience
  (params (ExperienceType :type String))
  ;[0.9734 0.1356 0.1356] Server: Base Experience List
  ;;[1 1 1 0.498] Server: Experience Base Events
  (Manager|Private|Maps|Remove|RemoveExperience ExperienceType))

(event Custom|Server_ClearExperience
  ;[0.9734 0.1356 0.1356] Server: Base Experience List
  ;;[1 1 1 0.498] Server: Experience Base Events
  (Manager|Private|Maps|Clear|ClearExperience))

(event EventBeginPlay
  ;[0.3916 1 0.3372] Event: Initialize Experience Bars
  (Utilities|FlowControl|Delay 0.1)
  (CallFunction|LoadTimer))

(fn CalculateRequiredExperience
  (params (LevelModifier :type Curve%20Float%20Object%20Reference) (Level :type Integer))
  ;[1 0.8228 0.1746] Calculate Required Experience
  (return (Math|Float|Round (select (Utilities|IsValid LevelModifier) (Math|Curves|GetFloatValue LevelModifier (Math|Conversions|ToFloat(Integer) Level)) (Math|Float|MakeLiteralFloat 1.0)))))

(fn GetExperience
  (params (Experience :type String))
  ;[0.3916 1 0.3372] Get Experience
  (bind (_returnvalue _value) (Manager|Private|Maps|Find|FindExperience Experience))
  (return _returnvalue _value))

(fn ModifyExperienceLevel
  (params (Experience :type String) (Calculation :type CalculationType%20Enum :default "NewEnumerator0") (Amount :type Integer))
  ;[0.9734 0.1356 0.1356] Modify Experience Level
  (bind (_returnvalue _value) (Manager|Private|Maps|Find|FindExperience Experience))
  (if _returnvalue
    (bind _structout (Utilities|Struct|SetmembersinExperienceList _value (select (.HasMaxLevel (Utilities|Struct|BreakExperienceList _value)) (Math|Integer|Clamp(Integer) (+ (.Level (Utilities|Struct|BreakExperienceList _value)) (Manager|Private|Math|CalculateValueModify(int) Calculation Amount)) 0 (.MaxLevel (Utilities|Struct|BreakExperienceList _value))) (Manager|Private|Math|ClampNoMax(int) (+ (.Level (Utilities|Struct|BreakExperienceList _value)) (Manager|Private|Math|CalculateValueModify(int) Calculation Amount))))))
    (Manager|Private|Maps|Add|AddExperience Experience _structout)
    (Interface|Experience|OnExperienceChanged Experience (.Level (Utilities|Struct|BreakExperienceList _value)) (select (.HasMaxLevel (Utilities|Struct|BreakExperienceList _value)) (Math|Integer|Clamp(Integer) (+ (.Level (Utilities|Struct|BreakExperienceList _value)) (Manager|Private|Math|CalculateValueModify(int) Calculation Amount)) 0 (.MaxLevel (Utilities|Struct|BreakExperienceList _value))) (Manager|Private|Math|ClampNoMax(int) (+ (.Level (Utilities|Struct|BreakExperienceList _value)) (Manager|Private|Math|CalculateValueModify(int) Calculation Amount)))))))

(fn BuildExperiences
  (bind _experiencebackup (Variables|Manager|Backup|GetExperienceBackup))
  ;[0.9734 0.1356 0.1356] Build Experiences
  (Utilities|HasMapElement _experiencebackup
    (:true
      (Manager|Private|Maps|Clear|ClearExperience)
      (bind _keys (Utilities|Map|Keys _experiencebackup))
      (for _array_element _keys
        (if (.ReturnValue (Utilities|Map|Find _experiencebackup _array_element))
          (Manager|Private|Maps|Add|AddExperience _array_element (Utilities|Struct|MakeExperienceList (.DisplayName (Utilities|Struct|BreakExperienceList (.Value (Utilities|Map|Find _experiencebackup _array_element)))) (.HasMaxLevel (Utilities|Struct|BreakExperienceList (.Value (Utilities|Map|Find _experiencebackup _array_element)))) (.MaxLevel (Utilities|Struct|BreakExperienceList (.Value (Utilities|Map|Find _experiencebackup _array_element)))) (Math|Integer|Clamp(Integer) (.Level (Utilities|Struct|BreakExperienceList (.Value (Utilities|Map|Find _experiencebackup _array_element)))) 0 (.MaxLevel (Utilities|Struct|BreakExperienceList (.Value (Utilities|Map|Find _experiencebackup _array_element))))) (.ExperienceAmount (Utilities|Struct|BreakExperienceList (.Value (Utilities|Map|Find _experiencebackup _array_element)))) (.LevelModifier (Utilities|Struct|BreakExperienceList (.Value (Utilities|Map|Find _experiencebackup _array_element))))))))
      (Default|CallExperiencesBuilded)
      (return))
    (:false
      (return))))

(fn InitializeExperienceManager
  (params (Experiences :type Map%20of%20Strings%20to%20Structs))
  ;[0.3916 1 0.3372] Initialize Experience Manager - Setup Experience
  (CallFunction|EventLoadExperiences Experiences))

(fn LoadExperiences
  (params (Experiences :type Map%20of%20Strings%20to%20Structs))
  ;[0.9734 0.1356 0.1356] Load Information - Initialize Experiences
  (Variables|Manager|Backup|SetExperienceBackup Experiences)
  (Interface|Experience|BuildExperiences))

(fn HasExperience
  (params (Experience :type String))
  ;[0.3916 1 0.3372] Has Experience
  (return (Utilities|Map|Contains (Variables|Default|GetExperience) Experience)))

(fn SetExperienceLevelModifier
  (params (Experience :type String) (LevelModifier :type Curve%20Float%20Object%20Reference))
  ;[0.9734 0.1356 0.1356] Set Experience Level Modifier
  (bind (_returnvalue _value) (Manager|Private|Maps|Find|FindExperience Experience))
  (if _returnvalue
    (bind _structout (Utilities|Struct|SetmembersinExperienceList _value LevelModifier))
    (Manager|Private|Maps|Add|AddExperience Experience _structout)
    (if (> (.ExperienceAmount (Utilities|Struct|BreakExperienceList _structout)) (Manager|Private|Math|CalculateRequiredExperience (.LevelModifier (Utilities|Struct|BreakExperienceList _structout)) (.Level (Utilities|Struct|BreakExperienceList _structout))))
      (Interface|Experience|ModifyExperienceAmount Experience "NewEnumerator0"))))

(fn ModifyExperienceAmount
  (params (Experience :type String) (Calculation :type CalculationType%20Enum :default "NewEnumerator0") (Amount :type Integer))
  ;[0.9734 0.1356 0.1356] Modify Experience Amount
  (LocalVariables|SetLocalAmount (Manager|Private|Math|ClampNoMax(int) Amount))
  (bind (_returnvalue _value) (Manager|Private|Maps|Find|FindExperience Experience :!label _label))
  (if _returnvalue
    (LocalVariables|SetLocalHasMaxLevel (.HasMaxLevel (Utilities|Struct|BreakExperienceList _value)))
    (LocalVariables|SetLocalMaxLevel (.MaxLevel (Utilities|Struct|BreakExperienceList _value)))
    (LocalVariables|SetLocalLevel (.Level (Utilities|Struct|BreakExperienceList _value)))
    (LocalVariables|SetLocalExperienceAmount (.ExperienceAmount (Utilities|Struct|BreakExperienceList _value)))
    (if (Utilities|Select :Index Calculation :NewEnumerator0 (>= (+ (Utilities|Struct|BreakExperienceList _value) (LocalVariables|GetLocalAmount)) (Interface|Experience|GetRequiredExperience Experience)) :NewEnumerator1 (<= (- (Utilities|Struct|BreakExperienceList _value) (LocalVariables|GetLocalAmount)) 0))
      (LocalVariables|SetLocalAmount (Utilities|Select :Index Calculation :NewEnumerator0 (- (+ (LocalVariables|GetLocalExperienceAmount) (LocalVariables|GetLocalAmount)) (Interface|Experience|GetRequiredExperience Experience)) :NewEnumerator1 (Math|Integer|Absolute(Integer) (- (LocalVariables|GetLocalExperienceAmount) (LocalVariables|GetLocalAmount)))))
      (bind _structout (Utilities|Struct|SetmembersinExperienceList _value (Math|Integer|Clamp(Integer) (Utilities|Select :Index Calculation :NewEnumerator0 (+ (LocalVariables|GetLocalLevel) 1) :NewEnumerator1 (- (LocalVariables|GetLocalLevel) 1)) 0 (select (LocalVariables|GetLocalHasMaxLevel) (LocalVariables|GetLocalMaxLevel) (Manager|Private|Math|ClampNoMax(int) (Utilities|Select :Index Calculation :NewEnumerator0 (+ (LocalVariables|GetLocalLevel) 1) :NewEnumerator1 (- (LocalVariables|GetLocalLevel) 1))))) (Utilities|Select :Index Calculation :NewEnumerator0 (select (== (LocalVariables|GetLocalLevel) (LocalVariables|GetLocalMaxLevel)) (LocalVariables|GetLocalAmount) 0) :NewEnumerator1 (select (== (LocalVariables|GetLocalLevel) 0) (LocalVariables|GetLocalAmount) (Interface|Experience|GetPreviousLevelRequioredExperience Experience)))))
      (Manager|Private|Maps|Add|AddExperience Experience _structout)
      (if (> (LocalVariables|GetLocalAmount) 0)
        (goto _label)
        (else
          (return)))
      (else
        (Interface|Experience|SetExperienceAmount Experience (Utilities|Select :Index Calculation :NewEnumerator0 (+ (LocalVariables|GetLocalExperienceAmount) (LocalVariables|GetLocalAmount)) :NewEnumerator1 (- (LocalVariables|GetLocalExperienceAmount) (LocalVariables|GetLocalAmount))))
        (return)))
    (else
      (return))))

(fn SetExperienceLevel
  (params (Experience :type String) (Amount :type Integer))
  ;[0.9734 0.1356 0.1356] Set Experience Level
  (bind (_returnvalue _value) (Manager|Private|Maps|Find|FindExperience Experience))
  (if _returnvalue
    (bind _structout (Utilities|Struct|SetmembersinExperienceList _value (select (.HasMaxLevel (Utilities|Struct|BreakExperienceList _value)) (Math|Integer|Clamp(Integer) Amount 0 (.MaxLevel (Utilities|Struct|BreakExperienceList _value))) (Manager|Private|Math|ClampNoMax(int) Amount))))
    (Manager|Private|Maps|Add|AddExperience Experience _structout)
    (Interface|Experience|OnExperienceChanged Experience (.Level (Utilities|Struct|BreakExperienceList _value)) (select (.HasMaxLevel (Utilities|Struct|BreakExperienceList _value)) (Math|Integer|Clamp(Integer) Amount 0 (.MaxLevel (Utilities|Struct|BreakExperienceList _value))) (Manager|Private|Math|ClampNoMax(int) Amount)))))

(fn SetExperienceAmount
  (params (Experience :type String) (Amount :type Integer))
  ;[0.9734 0.1356 0.1356] Set Experience Amount
  (bind (_returnvalue _value) (Manager|Private|Maps|Find|FindExperience Experience))
  (if _returnvalue
    (bind _structout (Utilities|Struct|SetmembersinExperienceList _value (Math|Integer|Clamp(Integer) Amount 0 (Interface|Experience|GetRequiredExperience Experience))))
    (Manager|Private|Maps|Add|AddExperience Experience _structout)))

(fn FindExperience
  (params (ExperienceType :type String))
  (bind _experience (Variables|Default|GetExperience))
  (bind (_value _returnvalue) (Utilities|Map|Find _experience ExperienceType))
  ;[0.3968 0.7305 1] Find Experience
  (return _returnvalue _value))

(fn AddExperience
  (params (ExperienceType :type String) (Values :type Experience%20List%20Structure))
  ;[0.3968 0.7305 1] Add Experience
  (Utilities|CanCreateExperience ExperienceType
    (:true
      (Utilities|Map|Add (Variables|Default|GetExperience) ExperienceType Values)
      (return))
    (:false
      (return))))

(fn RemoveExperience
  (params (ExperienceType :type String))
  ;[0.3968 0.7305 1] Remove Experience
  (bind _returnvalue (Utilities|Map|Remove (Variables|Default|GetExperience) ExperienceType))
  (return _returnvalue))

(fn GetExperienceList
  ;[0.3916 1 0.3372] Get Experience List
  (return (Variables|Default|GetExperience)))

(fn BuildSpecificExperience
  (params (ExperienceType :type String))
  (bind _experiencebackup (Variables|Manager|Backup|GetExperienceBackup))
  (bind _value (Utilities|Map|Find _experiencebackup ExperienceType))
  (bind (_displayname _hasmaxlevel _maxlevel _level _experienceamount _levelmodifier) (Utilities|Struct|BreakExperienceList _value))
  ;[0.9734 0.1356 0.1356] Build Specific Experience
  (Manager|Private|Maps|Remove|RemoveExperience ExperienceType)
  (Manager|Private|Maps|Add|AddExperience ExperienceType (Utilities|Struct|MakeExperienceList _displayname _hasmaxlevel _maxlevel (Math|Integer|Clamp(Integer) _level 0 _maxlevel) _experienceamount _levelmodifier))
  (Default|CallSpecificExperienceBuilded ExperienceType))

(fn ClearExperience
  ;[0.3968 0.7305 1] Clear Experience
  (Utilities|Map|Clear (Variables|Default|GetExperience)))

(fn ClampNoMax(int)
  (params (Value :type Integer))
  ;[1 0.8228 0.1746] Clamp No Max
  (return (Math|Integer|Clamp(Integer) Value 0 (Math|Integer|Absolute(Integer) Value))))

(fn GetPreviousLevelRequioredExperience
  (params (Experience :type String))
  ;[0.3916 1 0.3372] Get Previous Level Required Experience
  (bind (_returnvalue _value) (Manager|Private|Maps|Find|FindExperience))
  (if _returnvalue
    (return (select (Utilities|IsValid (.LevelModifier (Utilities|Struct|BreakExperienceList _value))) (Math|Integer|Clamp(Integer) (Math|Float|Ceil (Math|Curves|GetFloatValue (.LevelModifier (Utilities|Struct|BreakExperienceList _value)) (Math|Conversions|ToFloat(Integer) (Manager|Private|Math|ClampNoMax(int) (- (.Level (Utilities|Struct|BreakExperienceList _value)) 1))))) 1 (Manager|Private|Math|ClampNoMax(int) (Math|Float|Ceil (Math|Curves|GetFloatValue (.LevelModifier (Utilities|Struct|BreakExperienceList _value)) (Math|Conversions|ToFloat(Integer) (Manager|Private|Math|ClampNoMax(int) (- (.Level (Utilities|Struct|BreakExperienceList _value)) 1))))))) 1))
    (else
      (return 1))))

(fn GetNextLevelRequiredExperience
  (params (Experience :type String))
  ;[0.3916 1 0.3372] Get Next Level Required Experience
  (bind (_returnvalue _value) (Manager|Private|Maps|Find|FindExperience Experience))
  (if _returnvalue
    (return (select (Utilities|IsValid (.LevelModifier (Utilities|Struct|BreakExperienceList _value))) (Math|Integer|Clamp(Integer) (Math|Float|Ceil (Math|Curves|GetFloatValue (.LevelModifier (Utilities|Struct|BreakExperienceList _value)) (Math|Conversions|ToFloat(Integer) (Manager|Private|Math|ClampNoMax(int) (+ (.Level (Utilities|Struct|BreakExperienceList _value)) 1))))) 1 (Manager|Private|Math|ClampNoMax(int) (Math|Float|Ceil (Math|Curves|GetFloatValue (.LevelModifier (Utilities|Struct|BreakExperienceList _value)) (Math|Conversions|ToFloat(Integer) (Manager|Private|Math|ClampNoMax(int) (+ (.Level (Utilities|Struct|BreakExperienceList _value)) 1))))))) 1))
    (else
      (return 1))))

(fn GetRequiredExperience
  (params (Experience :type String))
  ;[0.3916 1 0.3372] Get Required Experience
  (bind (_returnvalue _value) (Manager|Private|Maps|Find|FindExperience Experience))
  (if _returnvalue
    (return (select (Utilities|IsValid (.LevelModifier (Utilities|Struct|BreakExperienceList _value))) (Math|Integer|Clamp(Integer) (Math|Float|Ceil (Math|Curves|GetFloatValue (.LevelModifier (Utilities|Struct|BreakExperienceList _value)) (Math|Conversions|ToFloat(Integer) (.Level (Utilities|Struct|BreakExperienceList _value))))) 1 (Manager|Private|Math|ClampNoMax(int) (Math|Float|Ceil (Math|Curves|GetFloatValue (.LevelModifier (Utilities|Struct|BreakExperienceList _value)) (Math|Conversions|ToFloat(Integer) (.Level (Utilities|Struct|BreakExperienceList _value))))))) 1))
    (else
      (return 1))))

(fn CalculateValueModify(int)
  (params (Calculation :type CalculationType%20Enum :default "NewEnumerator0") (InputValue :type Integer))
  (bind _returnvalue (Math|Integer|Absolute(Integer) InputValue))
  ;[1 0.8228 0.1746] Calculate Value Modify - Add / Subtract Value (int)
  (return (Utilities|Select :Index Calculation :NewEnumerator0 _returnvalue :NewEnumerator1 (* _returnvalue -1))))

(fn OnExperienceChanged
  (params (ExperienceType :type String) (Value :type Integer) (NewValue :type Integer))
  ;[0.3968 0.7305 1] On Experience Changed
  (Utilities|FlowControl|Sequence
    (:then_0
      (Utilities|OnExperienceIncreased ExperienceType Value NewValue
        (:IsIncreasded
          _)
        (:IsNotIncreased
          _))
      (Utilities|OnExperienceFull ExperienceType))
    (:then_1
      (Utilities|OnExperienceDecreased ExperienceType Value NewValue
        (:IsIncreasded
          _)
        (:IsNotIncreased
          _))
      (Utilities|OnExperienceEmpty ExperienceType))))