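; Score manager component that keeps a map of named integer scores, each with a display name and optional min and max limits.
; Loading stores a backup map, from which all scores or a single one are rebuilt, followed by a notification call.
; Server-prefixed events wrap the add, remove, clear, build and edit functions.
; Edits write the struct back into the map, and limit changes re-clamp the value by adding zero.
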(event Custom|Server_SetScoreValue
  (params (Score :type String) (Value :type Integer))
  ;[0.9734 0.1356 0.1356] Server: Score Events
  ;;[1 1 1 0.498] Score Amount
  (Interface|Score|SetScoreValue Score Value))

(event Custom|Server_RemoveScore
  (params (ScoreType :type String))
  ;[0.9734 0.1356 0.1356] Server: Base Score List
  ;;[1 1 1 0.498] Server: Score Base Events
  (Manager|Private|Maps|Remove|RemoveScore ScoreType))

(event Custom|Server_SetScoreDisplayName
  (params (Score :type String) (Name :type Name))
  ;[0.9734 0.1356 0.1356] Server: Score Events
  ;;[1 1 1 0.498] Score Name
  (Interface|Score|SetScoreDisplayName Score Name))

(event Custom|Server_ModifyScoreValue
  (params (Score :type String) (Calculation :type CalculationType%20Enum :default "NewEnumerator0") (Value :type Integer))
  ;[0.9734 0.1356 0.1356] Server: Score Events
  ;;[1 1 1 0.498] Score Amount
  (Interface|Score|ModifyScoreValue Score Calculation Value))

(event Custom|Server_SetScoreMaxValue
  (params (Score :type String) (Value :type Integer))
  ;[0.9734 0.1356 0.1356] Server: Score Events
  ;;[1 1 1 0.498] Max Score Value
  (Interface|Score|SetScoreMaxValue Score Value))

(event Custom|Server_ModifyScoreMaxValue
  (params (Score :type String) (Calculation :type CalculationType%20Enum :default "NewEnumerator0") (Value :type Integer))
  ;[0.9734 0.1356 0.1356] Server: Score Events
  ;;[1 1 1 0.498] Max Score Value
  (Interface|Score|ModifyScoreMaxValue Score Calculation Value))

(event Custom|Server_ClearScore
  ;[0.9734 0.1356 0.1356] Server: Base Score List
  ;;[1 1 1 0.498] Server: Score Base Events
  (Manager|Private|Maps|Clear|ClearScore))

(event Custom|Event_InitializeScoreManager
  (params (Scores :type Map%20of%20Strings%20to%20Structs))
  ;[0.3916 1 0.3372] Event: Initialize Scores
  (Manager|Public|InitializeScoreManager Scores))

(event Custom|Server_SetScoreMinValue
  (params (Score :type String) (Value :type Integer))
  ;[0.9734 0.1356 0.1356] Server: Score Events
  ;;[1 1 1 0.498] Min Score Value
  (Interface|Score|SetScoreMinValue Score Value))

(event Custom|Server_ModifyScoreMinValue
  (params (Score :type String) (Calculation :type CalculationType%20Enum :default "NewEnumerator0") (Value :type Integer))
  ;[0.9734 0.1356 0.1356] Server: Score Events
  ;;[1 1 1 0.498] Min Score Value
  (Interface|Score|ModifyScoreMinValue Score Calculation Value))

(event Custom|Server_SetScoreHasMaxValue
  (params (Score :type String) (HasMaxValue :type Boolean))
  ;[0.9734 0.1356 0.1356] Server: Score Events
  ;;[1 1 1 0.498] Max Score Value
  (Interface|Score|SetScoreHasMaxValue Score HasMaxValue))

(event Custom|Server_SetScoreHasMinValue
  (params (Score :type String) (HasMinValue :type Boolean))
  ;[0.9734 0.1356 0.1356] Server: Score Events
  ;;[1 1 1 0.498] Min Score Value
  (Interface|Score|SetScoreHasMinValue Score HasMinValue))

(event Custom|Event_LoadScores
  (params (Scores :type Map%20of%20Strings%20to%20Structs))
  ;[0.9734 0.1356 0.1356] Event: Load Scores
  (Manager|Public|LoadScores Scores))

(event Custom|Server_BuildScores
  ;[0.9734 0.1356 0.1356] Server: Base Score List
  ;;[1 1 1 0.498] Server: Score Base Events
  (Interface|Score|BuildScores))

(event Custom|Server_AddScore
  (params (ScoreType :type String) (Values :type Score%20List%20Structure))
  ;[0.9734 0.1356 0.1356] Server: Base Score List
  ;;[1 1 1 0.498] Server: Score Base Events
  (Manager|Private|Maps|Add|AddScore ScoreType Values))

(event Custom|Server_BuildSpecificScore
  (params (ScoreType :type String))
  ;[0.9734 0.1356 0.1356] Server: Base Score List
  ;;[1 1 1 0.498] Server: Score Base Events
  (Interface|Score|BuildSpecificScore ScoreType))

(event EventBeginPlay
  ;[0.3916 1 0.3372] Event: Initialize Scores
  (Utilities|FlowControl|Delay 0.1)
  (CallFunction|LoadTimer))

(fn InitializeScoreManager
  (params (Scores :type Map%20of%20Strings%20to%20Structs))
  ;[0.3916 1 0.3372] Initialize Score Manager - Setup Scores
  (CallFunction|EventLoadScores Scores))

(fn LoadScores
  (params (Scores :type Map%20of%20Strings%20to%20Structs))
  ;[0.9734 0.1356 0.1356] Load Scores - Initialize Scores
  (Variables|Manager|Backup|SetScoreBackup Scores)
  (Interface|Score|BuildScores))

(fn FindScore
  (params (ScoreType :type String))
  (bind _score (Variables|Default|GetScore))
  (bind (_value _returnvalue) (Utilities|Map|Find _score ScoreType))
  ;[0.3968 0.7305 1] Find Score
  (return _returnvalue _value))

(fn AddScore
  (params (ScoreType :type String) (Values :type Score%20List%20Structure))
  ;[0.3968 0.7305 1] Add Score
  (Utilities|CanCreateScore ScoreType
    (:true
      (Utilities|Map|Add (Variables|Default|GetScore) ScoreType Values)
      (return))
    (:false
      (return))))

(fn RemoveScore
  (params (ScoreType :type String))
  ;[0.3968 0.7305 1] Remove Score
  (bind _returnvalue (Utilities|Map|Remove (Variables|Default|GetScore) ScoreType))
  (return _returnvalue))

(fn GetScoreList
  ;[0.3916 1 0.3372] Get Score List
  (return (Variables|Default|GetScore)))

(fn ClearScore
  ;[0.3968 0.7305 1] Clear Score
  (Utilities|Map|Clear (Variables|Default|GetScore)))

(fn GetScore
  (params (ScoreType :type String))
  ;[0.3916 1 0.3372] Get Score
  (bind (_returnvalue _value) (Manager|Private|Maps|Find|FindScore ScoreType))
  (return _returnvalue _value))

(fn HasScore
  (params (ScoreType :type String))
  ;[0.3916 1 0.3372] Has Score
  (return (Utilities|Map|Contains (Variables|Default|GetScore) ScoreType)))

(fn BuildScores
  (bind _scorebackup (Variables|Manager|Backup|GetScoreBackup))
  ;[0.9734 0.1356 0.1356] Build Scores
  (Utilities|HasMapElement _scorebackup
    (:true
      (Manager|Private|Maps|Clear|ClearScore)
      (bind _keys (Utilities|Map|Keys _scorebackup))
      (for _array_element _keys
        (if (.ReturnValue (Utilities|Map|Find _scorebackup _array_element))
          (Manager|Private|Maps|Add|AddScore _array_element (Utilities|Struct|MakeScoreList (.DisplayName (Utilities|Struct|BreakScoreList (.Value (Utilities|Map|Find _scorebackup _array_element)))) (.HasMaxValue (Utilities|Struct|BreakScoreList (.Value (Utilities|Map|Find _scorebackup _array_element)))) (.MaxValue (Utilities|Struct|BreakScoreList (.Value (Utilities|Map|Find _scorebackup _array_element)))) (.HasMinValue (Utilities|Struct|BreakScoreList (.Value (Utilities|Map|Find _scorebackup _array_element)))) (.MinValue (Utilities|Struct|BreakScoreList (.Value (Utilities|Map|Find _scorebackup _array_element)))) (Math|Integer|Clamp(Integer) (.Value (Utilities|Struct|BreakScoreList (.Value (Utilities|Map|Find _scorebackup _array_element)))) (Manager|Private|Math|SetScoreClampMin (.HasMinValue (Utilities|Struct|BreakScoreList (.Value (Utilities|Map|Find _scorebackup _array_element)))) (.MinValue (Utilities|Struct|BreakScoreList (.Value (Utilities|Map|Find _scorebackup _array_element)))) (.Value (Utilities|Struct|BreakScoreList (.Value (Utilities|Map|Find _scorebackup _array_element))))) (Manager|Private|Math|SetScoreClampMax (.HasMaxValue (Utilities|Struct|BreakScoreList (.Value (Utilities|Map|Find _scorebackup _array_element)))) (.MaxValue (Utilities|Struct|BreakScoreList (.Value (Utilities|Map|Find _scorebackup _array_element)))) (.Value (Utilities|Struct|BreakScoreList (.Value (Utilities|Map|Find _scorebackup _array_element))))))))))
      (Default|CallScoresBuilded)
      (return))
    (:false
      (return))))

(fn BuildSpecificScore
  (params (ScoreType :type String))
  (bind _scorebackup (Variables|Manager|Backup|GetScoreBackup))
  (bind _value (Utilities|Map|Find _scorebackup ScoreType))
  (bind (_displayname _hasmaxvalue _maxvalue _hasminvalue _minvalue _value_2) (Utilities|Struct|BreakScoreList _value))
  ;[0.9734 0.1356 0.1356] Build Specific Score
  (Manager|Private|Maps|Remove|RemoveScore ScoreType)
  (Manager|Private|Maps|Add|AddScore ScoreType (Utilities|Struct|MakeScoreList _displayname _hasmaxvalue _maxvalue _hasminvalue _minvalue (Math|Integer|Clamp(Integer) _value_2 (Manager|Private|Math|SetScoreClampMin _hasminvalue _minvalue _value_2) (Manager|Private|Math|SetScoreClampMax _hasmaxvalue _maxvalue _value_2))))
  (Default|CallSpecificScoreBuilded ScoreType))

(fn SetScoreValue
  (params (Score :type String) (Value :type Integer))
  ;[0.9734 0.1356 0.1356] Set Score Value
  (bind (_returnvalue _value) (Manager|Private|Maps|Find|FindScore Score))
  (if _returnvalue
    (bind _structout (Utilities|Struct|SetmembersinScoreList _value (Math|Integer|Clamp(Integer) Value (Manager|Private|Math|SetScoreClampMin (.HasMinValue (Utilities|Struct|BreakScoreList _value)) (.MinValue (Utilities|Struct|BreakScoreList _value)) Value) (Manager|Private|Math|SetScoreClampMax (.HasMaxValue (Utilities|Struct|BreakScoreList _value)) (.MaxValue (Utilities|Struct|BreakScoreList _value)) Value))))
    (Manager|Private|Maps|Add|AddScore Score _structout)))

(fn ModifyScoreValue
  (params (Score :type String) (Calculation :type CalculationType%20Enum :default "NewEnumerator0") (Value :type Integer))
  ;[0.9734 0.1356 0.1356] Modify Score Value
  (bind (_returnvalue _value) (Manager|Private|Maps|Find|FindScore Score))
  (if _returnvalue
    (bind _structout (Utilities|Struct|SetmembersinScoreList _value (Math|Integer|Clamp(Integer) (+ (.Value (Utilities|Struct|BreakScoreList _value)) (Manager|Private|Math|CalculateValueModify Calculation Value)) (Manager|Private|Math|SetScoreClampMin (.HasMinValue (Utilities|Struct|BreakScoreList _value)) (.MinValue (Utilities|Struct|BreakScoreList _value)) (+ (.Value (Utilities|Struct|BreakScoreList _value)) (Manager|Private|Math|CalculateValueModify Calculation Value))) (Manager|Private|Math|SetScoreClampMax (.HasMaxValue (Utilities|Struct|BreakScoreList _value)) (.MaxValue (Utilities|Struct|BreakScoreList _value)) (+ (.Value (Utilities|Struct|BreakScoreList _value)) (Manager|Private|Math|CalculateValueModify Calculation Value))))))
    (Manager|Private|Maps|Add|AddScore Score _structout)))

(fn SetScoreHasMaxValue
  (params (Score :type String) (HasMaxValue :type Boolean))
  ;[0.9734 0.1356 0.1356] Set Score Has Max Value
  (bind (_returnvalue _value) (Manager|Private|Maps|Find|FindScore Score))
  (if _returnvalue
    (bind _structout (Utilities|Struct|SetmembersinScoreList _value HasMaxValue))
    (Manager|Private|Maps|Add|AddScore Score _structout)
    (Interface|Score|ModifyScoreValue Score "NewEnumerator0")))

(fn SetScoreMaxValue
  (params (Score :type String) (Value :type Integer))
  ;[0.9734 0.1356 0.1356] Set Score Max Value
  (bind (_returnvalue _value) (Manager|Private|Maps|Find|FindScore Score))
  (if _returnvalue
    (bind _structout (Utilities|Struct|SetmembersinScoreList _value (Math|Integer|Clamp(Integer) Value (Math|Integer|SelectInt (.MinValue (Utilities|Struct|BreakScoreList _value)) (- Value 1) (.HasMinValue (Utilities|Struct|BreakScoreList _value))) (+ Value 1))))
    (Manager|Private|Maps|Add|AddScore Score _structout)
    (Interface|Score|ModifyScoreValue Score "NewEnumerator0")))

(fn ModifyScoreMaxValue
  (params (Score :type String) (Calculation :type CalculationType%20Enum :default "NewEnumerator0") (Value :type Integer))
  ;[0.9734 0.1356 0.1356] Modify Score Max Value
  (bind (_returnvalue _value) (Manager|Private|Maps|Find|FindScore Score))
  (if _returnvalue
    (bind _structout (Utilities|Struct|SetmembersinScoreList _value (+ (Utilities|Struct|BreakScoreList _value) (Manager|Private|Math|CalculateValueModify Calculation Value))))
    (Manager|Private|Maps|Add|AddScore Score _structout)
    (Interface|Score|ModifyScoreValue Score "NewEnumerator0")))

(fn SetScoreHasMinValue
  (params (Score :type String) (HasMinValue :type Boolean))
  ;[0.9734 0.1356 0.1356] Set Score Has Min Value
  (bind (_returnvalue _value) (Manager|Private|Maps|Find|FindScore Score))
  (if _returnvalue
    (bind _structout (Utilities|Struct|SetmembersinScoreList _value HasMinValue))
    (Manager|Private|Maps|Add|AddScore Score _structout)
    (Interface|Score|ModifyScoreValue Score "NewEnumerator0")))

(fn SetScoreMinValue
  (params (Score :type String) (Value :type Integer))
  ;[0.9734 0.1356 0.1356] Set Score Max Value
  (bind (_returnvalue _value) (Manager|Private|Maps|Find|FindScore Score))
  (if _returnvalue
    (bind _structout (Utilities|Struct|SetmembersinScoreList _value (Math|Integer|Clamp(Integer) Value (- Value 1) (Math|Integer|SelectInt (.MaxValue (Utilities|Struct|BreakScoreList _value)) (+ Value 1) (.HasMaxValue (Utilities|Struct|BreakScoreList _value))))))
    (Manager|Private|Maps|Add|AddScore Score _structout)
    (Interface|Score|ModifyScoreValue Score "NewEnumerator0")))

(fn ModifyScoreMinValue
  (params (Score :type String) (Calculation :type CalculationType%20Enum :default "NewEnumerator0") (Value :type Integer))
  ;[0.9734 0.1356 0.1356] Modify Score Min Value
  (bind (_returnvalue _value) (Manager|Private|Maps|Find|FindScore Score))
  (if _returnvalue
    (bind _structout (Utilities|Struct|SetmembersinScoreList _value (+ (Utilities|Struct|BreakScoreList _value) (Manager|Private|Math|CalculateValueModify Calculation Value))))
    (Manager|Private|Maps|Add|AddScore Score _structout)
    (Interface|Score|ModifyScoreValue Score "NewEnumerator0")))

(fn ClampNoMax
  (params (Value :type Integer))
  ;[1 0.8228 0.1746] Clamp No Max
  (return (Math|Integer|Clamp(Integer) Value 0 (Math|Integer|Absolute(Integer) Value))))

(fn CalculateValueModify
  (params (Calculation :type CalculationType%20Enum :default "NewEnumerator0") (InputValue :type Integer))
  (bind _returnvalue (Math|Integer|Absolute(Integer) InputValue))
  ;[1 0.8228 0.1746] Calculate Value Modify - Add / Subtract Value (int)
  (return (Utilities|Select :Index Calculation :NewEnumerator0 _returnvalue :NewEnumerator1 (* _returnvalue -1))))

(fn SetScoreClampMax
  (params (HasMaxValue :type Boolean) (MaxValue :type Integer) (Value :type Integer))
  ;[1 0.8228 0.1746] Clamp No Max
  (return (select HasMaxValue MaxValue (+ Value 1))))

(fn SetScoreClampMin
  (params (HasMinValue :type Boolean) (MinValue :type Integer) (Value :type Integer))
  ;[1 0.8228 0.1746] Clamp No Min
  (return (select HasMinValue MinValue (- Value 1))))

(fn SetScoreDisplayName
  (params (Score :type String) (Name :type Name))
  ;[0.9734 0.1356 0.1356] Set Score Display Name
  (bind (_returnvalue _value) (Manager|Private|Maps|Find|FindScore Score))
  (if _returnvalue
    (bind _structout (Utilities|Struct|SetmembersinScoreList _value Name))
    (Manager|Private|Maps|Add|AddScore Score _structout)))