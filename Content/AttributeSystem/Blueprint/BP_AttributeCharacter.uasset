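; Demo character for the attribute system that forwards damage to its controller and supports toggling a physics ragdoll.
; AnyDamage passes its full payload to the controller's TakeDamage.
; SetCharacterPhysics switches between a simulated mesh with an ignoring capsule and disabled movement, and a re-attached mesh with blocking collision and walking.
; While the pelvis simulates, Tick moves the actor to that socket, raised by the capsule half-height.
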(event EventTick
  (params (DeltaSeconds :type Float%20%28single-precision%29))
  ;[0.9734 0.1356 0.1356] Event Tick - (Demo)
  (Demo|SetCapsuleLocation) ; Sets the Capsule Location, when the Mesh is Simulating Physics
)

(event Game|Damage|EventAnyDamage
  (params (Damage :type Float%20%28single-precision%29) (DamageType :type Damage%20Type%20Object%20Reference) (InstigatedBy :type Controller%20Object%20Reference) (DamageCauser :type Actor%20Object%20Reference))
  ;[0.3185 0.6867 1] Event AnyDamage  - (Demo)
  (CallFunction|TakeDamage (Pawn|GetController) Damage DamageType InstigatedBy DamageCauser) ; Handles taking the Damage
)

(fn ConstructionScript)

(fn SetCapsuleLocation
  (bind _mesh (Variables|Character|GetMesh))
  (bind _pelvis (Variables|Demo|GetPelvis))
  ;[0.9734 0.1356 0.1356] Set Capsule Location  - Demo
  (if (Physics|IsSimulatingPhysics _mesh _pelvis)
    (Transformation|SetActorLocation (+ (Transformation|GetSocketLocation _mesh _pelvis) (Math|Vector|MakeVector 0.0 0.0 (Components|Capsule|GetScaledCapsuleHalfHeight (Variables|Collision|GetCapsuleComponent)))) false false)))

(fn SetCharacterPhysics
  (params (New%20Simulate :type Boolean))
  ;[0.9734 0.1356 0.1356] Set Character Physics - Demo
  (if New%20Simulate
    (Collision|SetCollisionResponsetoAllChannels (Variables|Collision|GetCapsuleComponent) "ECR_Ignore")
    (Pawn|Components|CharacterMovement|SetMovementMode (Variables|Character|GetCharacterMovement) "MOVE_None" 0)
    (Physics|SetSimulatePhysics (Variables|Character|GetMesh) true)
    (else
      (Physics|SetSimulatePhysics (Variables|Character|GetMesh) false)
      (Collision|SetCollisionResponsetoAllChannels (Variables|Collision|GetCapsuleComponent) "ECR_Block")
      (Class|SceneComponent|Attachto (Variables|Character|GetMesh) (Variables|Collision|GetCapsuleComponent) "None" "SnapToTarget" true)
      (Transformation|SetRelativeLocationAndRotation (Variables|Character|GetMesh) "0, 0,-96.000000" "0,-90.000000, 0" false false)
      (Transformation|SetRelativeLocation (Variables|MyCharacter|GetCameraBoom) "0, 0,10.000000" false false)
      (Pawn|Components|CharacterMovement|SetMovementMode (Variables|Character|GetCharacterMovement) "MOVE_Walking" 0))))