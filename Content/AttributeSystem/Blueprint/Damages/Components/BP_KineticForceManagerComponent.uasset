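; Actor component that damages its owning pawn when sudden velocity changes, such as impacts, exceed a G-force limit.
; On BeginPlay it caches the pawn's movement component and sets the tick interval.
; Each tick it measures speed on selectable axes and converts the change since the last update into G-force relative to gravity.
; Force above MaxGForce is scaled by KineticDamageRate and applied as damage of a configurable type.
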(event EventBeginPlay
  ;[0.3916 1 0.3372] Event Begin Play
  (CallFunction|InitializeComponent))

(event EventTick
  (params (DeltaSeconds :type Float%20%28single-precision%29))
  ;[0.9734 0.1356 0.1356] Event Tick
  (Variables|Default|SetDeltaSeconds DeltaSeconds)
  (bind _exceedsimpactforce (CallFunction|CalculateImpactForce))
  (if _exceedsimpactforce
    (CallFunction|CalculateKineticDamage)))

(fn CalculateImpactForce
  ;[0.9734 0.1356 0.1356] Calculate Impact Force
  (CallFunction|SetCurrentVelocity)
  (bind _output_get (Variables|Default|SetCurrentVelocity (Variables|Default|GetCurrentAxisVelocity)))
  (Variables|Default|SetCurrentG-Force (Math|Float|Absolute(Float) (/ (/ (- _output_get (Variables|Default|GetPreviousVelocity)) (Variables|Default|GetDeltaSeconds)) (Components|Movement|GetGravityZ (Variables|Components|GetMovementComponent)))))
  (Variables|Default|SetPreviousVelocity (Variables|Default|GetCurrentVelocity))
  (if (> (Variables|Default|GetCurrentG-Force) (Variables|Default|GetMaxG-Force))
    (return true)
    (else
      (return false))))

(fn InitializeComponent
  ;[0.3916 1 0.3372] Initialize Component
  (bind _aspawn (Utilities|Casting|CastToPawn (Components|GetOwner))
    (:then
      (bind _output_get (Variables|Components|SetPawnReference _aspawn))
      (Variables|Components|SetMovementComponent (Pawn|GetMovementComponent _output_get))
      (Class|ActorComponent|SetComponentTickInterval (Variables|Default|GetUpdateInterval))
      (return true))
    (:CastFailed
      (return false))))

(fn CalculateKineticDamage
  ;[0.9734 0.1356 0.1356] Calculate Kinetic Damage
  (LocalVariables|SetLocalDamage (* (- (Variables|Default|GetCurrentG-Force) (Variables|Default|GetMaxG-Force)) (Variables|Default|GetKineticDamageRate)))
  (Game|Damage|ApplyDamage (Variables|Components|GetPawnReference) (LocalVariables|GetLocalDamage) 0 0 (Variables|Default|GetDamageClass)) ; Apply damage to the character
)

(fn SetCurrentVelocity
  ;[0.9734 0.1356 0.1356] Set Current Velocity
  (Variables|Default|SetCurrentAxisVelocity (Math|Vector|VectorLength (Math|Vector|MakeVector (Math|Float|SelectFloat (.X (Math|Vector|BreakVector (Transformation|GetVelocity (Components|GetOwner)))) 0.0 (Variables|Default|GetUseX-Axis)) (Math|Float|SelectFloat (.Y (Math|Vector|BreakVector (Transformation|GetVelocity (Components|GetOwner)))) 0.0 (Variables|Default|GetUseY-Axis)) (Math|Float|SelectFloat (.Z (Math|Vector|BreakVector (Transformation|GetVelocity (Components|GetOwner)))) 0.0 (Variables|Default|GetUseZ-Axis))))))