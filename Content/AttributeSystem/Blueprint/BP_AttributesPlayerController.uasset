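; Player controller for the attribute system that drives the character, handles health-based death and revival, and toggles a debug window.
; After a short delay it caches character and HUD references, then feeds yaw-relative movement, look and jump input.
; An empty health bar increments the deaths score and enables character physics; pressing Jump while the mesh simulates disables it and refills health.
; P shows or hides the debug UI, switching input mode and cursor.
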(event BarEmpty(BarManagerComponent)
  (params (Bar :type String))
  ;[0.9734 0.1356 0.1356] On Bar Empty
  (if (Utilities|Enum|Equal(Enum) Bar "health")
    (Default|ModifyScoreValue (Variables|Default|GetScoreManagerComponent) "deaths" "NewEnumerator0" 1)
    (Default|SetCharacterPhysics (Variables|Default|GetCharacterReference) true)))

(event EventBeginPlay
  ;[0.3916 1 0.3372] Event Begin Play: Initialize Player
  (Utilities|FlowControl|Delay 0.1)
  (CallFunction|InitializePlayer))

(event Input|ActionEvents|InputActionJump
  (params (Key :type Key%20Structure))
  (bind _characterreference (Variables|Default|GetCharacterReference))
  (bind _barmanagercomponent (Variables|Default|GetBarManagerComponent))
  ;[1 0.8613 0.2188] Movement
  ;;[1 1 1 0.498] Input: Jump
  (:Pressed
    (Character|Jump _characterreference)
    (if (Physics|IsSimulatingPhysics (Variables|/Script/Engine.Character|GetMesh (Variables|Default|GetCharacterReference)) "None")
      (Default|SetCharacterPhysics (Variables|Default|GetCharacterReference) false)
      (Default|SetBarValue _barmanagercomponent "health" (Utilities|Struct|BreakBarList (.Values (Default|GetBar _barmanagercomponent "health"))) true true)))
  (:Released
    (Character|StopJumping _characterreference)))

(event Input|AxisEvents|InputAxisLookUp
  (params (AxisValue :type Float%20%28single-precision%29))
  ;[1 0.8613 0.2188] Movement
  ;;[1 1 1 0.498] Input: Mouse Movement
  (Class|PlayerController|AddPitchInput AxisValue))

(event Input|AxisEvents|InputAxisTurn
  (params (AxisValue :type Float%20%28single-precision%29))
  ;[1 0.8613 0.2188] Movement
  ;;[1 1 1 0.498] Input: Mouse Movement
  (Class|PlayerController|AddYawInput AxisValue))

(event Input|AxisEvents|InputAxisMoveForward
  (params (AxisValue :type Float%20%28single-precision%29))
  ;[1 0.8613 0.2188] Movement
  ;;[1 1 1 0.5] Input: Character Keyboard Movement
  (Utilities|CanMove
    (:true
      (Pawn|Input|AddMovementInput (Variables|Default|GetCharacterReference) (.ForwardVector (CallFunction|GetMovementVectors)) AxisValue false))))

(event Input|AxisEvents|InputAxisMoveRight
  (params (AxisValue :type Float%20%28single-precision%29))
  ;[1 0.8613 0.2188] Movement
  ;;[1 1 1 0.5] Input: Character Keyboard Movement
  (Utilities|CanMove
    (:true
      (Pawn|Input|AddMovementInput (Variables|Default|GetCharacterReference) (.RightVector (CallFunction|GetMovementVectors)) AxisValue false))))

(event Input|KeyboardEvents|P
  (params (Key :type Key%20Structure))
  (bind _self self)
  (bind _hud_reference (Variables|Default|GetHUD%20Reference))
  (bind _debug_window (Variables|/Ability/AttributeSystem/UI/Widgets/HUDLayout.HUDLayout_C|GetDebug_Window _hud_reference))
  ;[0.3185 0.6867 1] Input: Open/Close Debug Window
  (:Pressed
    (if (Variables|Default|GetIsDebugUIOpen)
      (Default|SetDebugVisibility _debug_window "Collapsed")
      ;[0.3185 0.6867 1] Input: Set UI Mode
      (Input|SetInputModeGameOnly _self)
      (Variables|Default|SetbShowMouseCursor false)
      (Variables|Default|SetIsDebugUIOpen false)
      (else
        (Default|SetDebugVisibility _debug_window "SelfHitTestInvisible")
        (Input|SetInputModeGameandUI _self (Variables|Default|GetHUD%20Reference) "DoNotLock" true)
        (Variables|Default|SetbShowMouseCursor true)
        (Variables|Default|SetIsDebugUIOpen true)))))

(fn ConstructionScript)

(fn InitializePlayer
  ;[0.9734 0.1356 0.1356] InitializePlayer: Cast to Character
  (bind _asbp_attribute_character (Utilities|Casting|CastToBP_AttributeCharacter (Pawn|GetControlledPawn)))
  (Variables|Default|SetCharacterReference _asbp_attribute_character) ; Get Character Reference
  ;[0.3916 1 0.3372] Client: Get HUD UI
  (bind _asbp_attribute_hud (Utilities|Casting|CastToBP_AttributeHUD (HUD|GetHUD)))
  (Variables|Default|SetHUD%20Reference (Variables|/Ability/AttributeSystem/Example/BP_AttributeHUD.BP_AttributeHUD_C|GetHUD%20Reference _asbp_attribute_hud)) ; Get HUD Widget Reference
)

(fn GetMovementVectors
  (bind _returnvalue (Pawn|GetControlRotation :!class /Script/Engine.Controller))
  (bind _yaw (Math|Rotator|BreakRotator _returnvalue))
  (bind _returnvalue_2 (Math|Rotator|MakeRotator 0.0 0.0 _yaw))
  ;[1 0.8115 0.1896] Get Movement Vectors
  (return (Math|Vector|GetForwardVector _returnvalue_2) (Math|Vector|GetRightVector _returnvalue_2)))