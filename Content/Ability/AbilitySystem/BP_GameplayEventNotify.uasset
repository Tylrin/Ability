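; An animation notify that sends a gameplay event to the owner of the mesh playing the animation.
; On trigger, it sends its configurable event tag and magnitude through the Gameplay Ability System, with the owner as instigator and target and the mesh and animation as optional objects.
; The notify displays the event tag as its name in the animation editor.
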(fn ReceivedNotify
  (params (MeshComp :type Skeletal%20Mesh%20Component%20Object%20Reference) (Animation :type Anim%20Sequence%20Base%20Object%20Reference))
  (bind _returnvalue (Components|GetOwner MeshComp))
  (Ability|SendGameplayEventtoActor (Components|GetOwner MeshComp) (Variables|Default|GetEventTag) (Utilities|Struct|MakeGameplayEventData (Variables|Default|GetEventTag) _returnvalue _returnvalue MeshComp Animation "()" "(GameplayTags=)" "(GameplayTags=)" (Variables|Default|GetEventMagnitude)))
  (return true))

(fn GetNotifyName
  (return (Utilities|String|ToString(Name) (GameplayTags|GetTagName (Variables|Default|GetEventTag)))))